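; BP_SlidingDoor is a key-locked door that slides open when interacted with.
; On BeginPlay it caches BP_GameMode, and Interact opens the door only if the game mode's Keys value exactly equals the door's KeyNumber, otherwise printing a message.
; The Door_Rotate timeline, despite its name, lerps the door's relative location from StartLocation to FinishLocation.
; The construction script applies the Material variable to the door mesh.
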(event EventBeginPlay
  (bind _asbp_game_mode (Utilities|Casting|CastToBP_GameMode (Game|GetGameMode)))
  (Variables|Default|SetAs%20BP%20Game%20Mode _asbp_game_mode))

(event EventInteract
  (if (== (Variables|/Game/BP_GameMode.BP_GameMode_C|GetKeys (Variables|Default|GetAs%20BP%20Game%20Mode)) (Variables|Default|GetKey%20Number))
    (bind _newtrack_0 (Timeline|Door_Rotate Play)
      (:Update
        (Transformation|SetRelativeLocation (Variables|Default|GetDoor) (Math|Vector|Lerp(Vector) (Variables|Default|GetStartLocation) (Variables|Default|GetFinishLocation) _newtrack_0) false false)))
    (else
      (Development|PrintString "You do not have the correct key."))))

(fn ConstructionScript
  (Rendering|Material|SetMaterial (Variables|Default|GetDoor) 0 (Variables|Default|GetMaterial)))