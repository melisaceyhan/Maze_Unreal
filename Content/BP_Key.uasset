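; BP_Key is an interactable key pickup that gives the player a numbered key.
; On BeginPlay it caches BP_GameMode, and its Construction Script applies a configurable material to the Key mesh.
; Interacting overwrites the game mode's Keys value with this key's KeyNumber, prints an acquired message using the matching name, then destroys the actor.
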(event EventInteract
  (bind _output_get (Variables|/Game/BP_GameMode.BP_GameMode_C|SetKeys (Variables|Default|GetAs%20BP%20Game%20Mode) (Variables|Default|GetKeyNumber)))
  (Development|PrintString (Utilities|String|Append "Key" (Utilities|Array|Get(acopy) (Variables|Default|GetNames) _output_get) "Acquired"))
  (Actor|DestroyActor))

(event EventBeginPlay
  (bind _asbp_game_mode (Utilities|Casting|CastToBP_GameMode (Game|GetGameMode)))
  (Variables|Default|SetAs%20BP%20Game%20Mode _asbp_game_mode))

(fn ConstructionScript
  (Rendering|Material|SetMaterial (Variables|Default|GetKey) 0 (Variables|Default|GetMaterial)))