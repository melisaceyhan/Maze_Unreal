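; BP_MazeCell is a single maze cell actor that builds its geometry in the Construction Script, with no active runtime logic.
; GridSize sets the floor footprint and wall thickness, while WallHeight sets how tall the walls are.
; Boolean flags add static mesh components for each wall and the ceiling, scaled from dimensions through SizeToCubeScale.
; A positive LightIntensity adds a colored point light at the cell's center at floor height.
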(event EventBeginPlay)

(event Collision|EventActorBeginOverlap
  (params (OtherActor :type Actor%20Object%20Reference)))

(event EventTick
  (params (DeltaSeconds :type Float%20%28single-precision%29)))

(fn ConstructionScript
  (bind _gridsize (Variables|Default|GetGridSize))
  (LocalVariables|SetWallLength _gridsize)
  (LocalVariables|SetWall%20Thickness (* _gridsize 0.1))
  (Transformation|SetRelativeScale3D (Variables|Default|GetFloor) (Utilities|SizetoCubeScale (Math|Vector|MakeVector (LocalVariables|GetWallLength) (LocalVariables|GetWallLength) (LocalVariables|GetWall%20Thickness))))
  (if (Variables|Default|GetWestWall)
    (AddComponent|AddStaticMeshComponent false (Math|Transform|MakeTransform (Math|Vector|MakeVector 0.0 0.0 0.0) "0, 0, 0" (Utilities|SizetoCubeScale (Math|Vector|MakeVector (LocalVariables|GetWallLength) (LocalVariables|GetWall%20Thickness) (Variables|Default|GetWallHeight))))))
  (if (Variables|Default|GetSouthWall)
    (AddComponent|AddStaticMeshComponent false (Math|Transform|MakeTransform (Math|Vector|MakeVector 0.0 0.0 0.0) "0, 0, 0" (Utilities|SizetoCubeScale (Math|Vector|MakeVector (LocalVariables|GetWall%20Thickness) (LocalVariables|GetWallLength) (Variables|Default|GetWallHeight))))))
  (if (Variables|Default|GetNorthWall)
    (AddComponent|AddStaticMeshComponent false (Math|Transform|MakeTransform (Math|Vector|MakeVector (- (LocalVariables|GetWallLength) (LocalVariables|GetWall%20Thickness)) 0.0 0.0) "0, 0, 0" (Utilities|SizetoCubeScale (Math|Vector|MakeVector (LocalVariables|GetWall%20Thickness) (LocalVariables|GetWallLength) (Variables|Default|GetWallHeight))))))
  (if (Variables|Default|GetEastWall)
    (AddComponent|AddStaticMeshComponent false (Math|Transform|MakeTransform (Math|Vector|MakeVector 0.0 (- (LocalVariables|GetWallLength) (LocalVariables|GetWall%20Thickness)) 0.0) "0, 0, 0" (Utilities|SizetoCubeScale (Math|Vector|MakeVector (LocalVariables|GetWallLength) (LocalVariables|GetWall%20Thickness) (Variables|Default|GetWallHeight))))))
  (if (Variables|Default|GetCeiling)
    (AddComponent|AddStaticMeshComponent false (Math|Transform|MakeTransform (Math|Vector|MakeVector 0.0 0.0 (Variables|Default|GetWallHeight)) "0, 0, 0" (Utilities|SizetoCubeScale (Math|Vector|MakeVector (LocalVariables|GetWallLength) (LocalVariables|GetWallLength) (LocalVariables|GetWall%20Thickness))))))
  (if (> (Variables|Default|GetLightIntensity) 0.0)
    (bind _returnvalue (AddComponent|AddPointLightComponent false (Math|Transform|MakeTransform (Math|Vector|MakeVector (* (LocalVariables|GetWallLength) 0.5) (* (LocalVariables|GetWallLength) 0.5) (* 0.0 (Variables|Default|GetWallHeight))) "0, 0, 0" "1.000000,1.000000,1.000000")))
    (Rendering|Components|Light|SetLightColor _returnvalue (Variables|Default|GetLightColor) true)
    (Rendering|Components|Light|SetIntensity _returnvalue (Variables|Default|GetLightIntensity))))